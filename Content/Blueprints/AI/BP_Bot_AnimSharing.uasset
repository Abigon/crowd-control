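; Bot actor that uses the Animation Sharing plugin to share skeletal animation on the UE4 Mannequin skeleton.
; On BeginPlay it creates the sharing manager from ASS_Bot if none exists, registers itself, and caches the AIRunComponent found on its controller.
; Every Tick it sets AnimSharedState to one of two values, depending on whether that component exists and reports movement.
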(event `self.ReceiveBeginPlay`
  (bind _returnvalue (`self.GetComponentByClass` (`self.GetController`) "/Script/Crowd.AIRunComponent"))
  (bind _returnvalue_2 (`AnimationSharingManager.GetAnimationSharingManager`))
  (`/Engine/EditorBlueprintResources/StandardMacros.IsValid` _returnvalue_2
    (:`Is Valid`
      _)
    (:`Is Not Valid`
      (`AnimationSharingManager.CreateAnimationSharingManager` "/Game/Blueprints/AI/AnimSharing/ASS_Bot.ASS_Bot")))
  (bind _returnvalue_3 (`AnimationSharingManager.GetAnimationSharingManager`))
  (`AnimationSharingManager.RegisterActorWithSkeletonBP` _returnvalue_3 self "/Game/Mannequin/Character/Mesh/UE4_Mannequin_Skeleton.UE4_Mannequin_Skeleton")
  (`/Engine/EditorBlueprintResources/StandardMacros.IsValid` _returnvalue
    (:`Is Valid`
      (set `self.AIRunComp` _returnvalue))))

(event `self.ReceiveTick`
  (params (DeltaSeconds :type "Float (single-precision)"))
  (bind _airuncomp (`self.AIRunComp`)
    (:`then`
      (if (`AIRunComponent.IsMoving` _airuncomp)
        (set `self.AnimSharedState` "NewEnumerator1")
        (else
          (set `self.AnimSharedState` "NewEnumerator0" :!label _label))))
    (:`else`
      (goto _label))))

(event `self.ReceiveEndPlay`
  (params (EndPlayReason :type "EEndPlayReason Enum" :default "Destroyed")))

(fn `UserConstructionScript`)